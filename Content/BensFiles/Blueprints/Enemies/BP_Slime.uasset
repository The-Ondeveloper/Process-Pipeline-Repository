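; BP_Slime is a slime enemy that chases the player and deals contact damage.
; Pawn sensing triggers an AI move toward the player character.
; Overlapping an actor starts a DoOnce-gated loop that damages it and shows a hit indicator widget every second until overlap ends.
; Taking damage animates a dynamic overlay material's opacity through a timeline, and the Health death event spawns a Niagara splatter near ground height.
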(event `self.PawnSensing.OnSeePawn`
  (params (Pawn :type "Pawn Object Reference"))
  ;[1 1 1] Follow Player
  (`self.FollowPawn`))

(event `FollowPawn`
  ;[1 1 1] Follow Player
  (`|AIMoveTo` self (0.0 0.0 0.0) (`GameplayStatics.GetPlayerCharacter` 0)))

(event `self.ReceiveActorBeginOverlap`
  (params (OtherActor :type "Actor Object Reference"))
  ;[1 0 0] Damage
  (set `self.Player_Ref` OtherActor)
  (`/Engine/EditorBlueprintResources/StandardMacros.DoOnce` false :!label _label
    (:`Completed`
      (`GameplayStatics.ApplyDamage` (`self.Player_Ref`) (`self.Damage`) :!label _label_2)
      (bind _returnvalue (`|CreateWidget` "/Game/BensFiles/Blueprints/UI/HitIndicator.HitIndicator_C"))
      (`UserWidget.AddToViewport` _returnvalue 0)
      (`KismetSystemLibrary.Delay` 1.0)
      (if (`self.IsOverlappingActor` (`self.Player_Ref`))
        (goto _label_2)
        (else
          (goto _label :!via `Reset`))))))

(event `self.ReceiveAnyDamage`
  (params (Damage :type "Float (single-precision)") (DamageType :type "DamageType Object Reference") (InstigatedBy :type "Controller Object Reference") (DamageCauser :type "Actor Object Reference"))
  ;[0 0 0] Hit Impact
  (bind _returnvalue (`KismetMaterialLibrary.CreateDynamicMaterialInstance` "/Game/BensFiles/Shaders/Enemies/M_Slime_Damage.M_Slime_Damage"))
  (bind _output_get (set `self.OverlayMat` _returnvalue))
  (`MeshComponent.SetOverlayMaterial` (`self.StaticMesh1`) _output_get)
  (bind (_direction _newtrack_0) (`Timeline|Timeline` :`NewTime` 1.0 :!via `PlayFromStart`)
    (:`Update`
      (`MaterialInstanceDynamic.SetScalarParameterValue` (`self.OverlayMat`) "Opacity" _newtrack_0))))

(event `self.Health.OnDeath`
  (bind (_returnvalue_x _returnvalue_y) (`KismetMathLibrary.BreakVector` (`self.K2_GetActorLocation`)))
  (`NiagaraFunctionLibrary.SpawnSystemAtLocation` "/Game/BensFiles/VFX/Niagara/NS_Slime_Splatter.NS_Slime_Splatter" (`KismetMathLibrary.MakeVector` _returnvalue_x _returnvalue_y 4.0)))

(fn `UserConstructionScript`)