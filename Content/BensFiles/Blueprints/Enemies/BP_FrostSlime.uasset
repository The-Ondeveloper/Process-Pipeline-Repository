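; BP_FrostSlime is an enemy slime that chases the player and deals contact damage.
; When pawn sensing sees any pawn, it issues an AI move toward player zero.
; Overlapping any actor stores it as PlayerRef, then a DoOnce-gated loop applies damage and adds a hit indicator widget.
; The loop repeats after a two-second delay while the overlap persists, then resets the gate.
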(event `self.PawnSensing.OnSeePawn`
  (params (Pawn :type "Pawn Object Reference"))
  ;[1 1 1] Follow Player
  (`self.FollowPawn`))

(event `FollowPawn`
  ;[1 1 1] Follow Player
  (`|AIMoveTo` self (0.0 0.0 0.0) (`GameplayStatics.GetPlayerCharacter` 0)))

(event `self.ReceiveActorBeginOverlap`
  (params (OtherActor :type "Actor Object Reference"))
  ;[1 0 0] Damage
  (set `self.Player_Ref` OtherActor)
  (`/Engine/EditorBlueprintResources/StandardMacros.DoOnce` false :!label _label
    (:`Completed`
      (`GameplayStatics.ApplyDamage` (`self.Player_Ref`) (`self.Damage`) :!label _label_2)
      (bind _returnvalue (`|CreateWidget` "/Game/BensFiles/Blueprints/UI/HitIndicator.HitIndicator_C"))
      (`UserWidget.AddToViewport` _returnvalue 0)
      (`KismetSystemLibrary.Delay` 2.0)
      (if (`self.IsOverlappingActor` (`self.Player_Ref`))
        (goto _label_2)
        (else
          (goto _label :!via `Reset`))))))

(fn `UserConstructionScript`)