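; First-person player character with movement, stamina-gated sprint and dodge, item pickup and inventory.
; Health, Stamina, Mana and Inventory components fire events that update the HUD stat bars, pouch and toggleable inventory menu.
; A looping timer sphere-traces from the camera for BPI_DS_Item actors, showing a pickup prompt and feeding the interact input.
; Equipped item changes async-load the held item class and attach a new instance to the hand socket.
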(event `self.ReceiveBeginPlay`
  (bind _playerui (`self.PlayerUI`))
  ;[0.4072 0.04817 0.2542] Initialises the Player UI and Stat Bars
  (bind _returnvalue (`|CreateWidget` "/Game/SeddonsContent/UI/GeneralUI/BPW_DS_PlayerUI.BPW_DS_PlayerUI_C"))
  (bind _output_get (set `self.PlayerUI` _returnvalue))
  (`/Game/SeddonsContent/UI/GeneralUI/BPW_DS_PlayerUI.Set Stat Bar Max Stats` _output_get (`/Game/SeddonsContent/Components/Stats/Health.Maxhealth` (`self.Health`)) (`/Game/SeddonsContent/Components/Stats/Stamina.MaxStamina` (`self.Stamina`)) (`/Game/SeddonsContent/Components/Stats/Mana.MaxMana` (`self.Mana`)))
  (`UserWidget.AddToViewport` _playerui 0)
  (`/Game/SeddonsContent/UI/InventoryUI/BPW_DS_InventoryPanelUI.Initalise slots` (`/Game/SeddonsContent/UI/GeneralUI/BPW_DS_PlayerUI.Pouch` _playerui) (`/Game/SeddonsContent/Components/Items/Inventory.PouchSize` (`self.Inventory`)))
  ;[0.4072 0.04817 0.2542] Initialises UI for looking at pick up items
  (`self.Start Raycast`)
  (bind _returnvalue_2 (`|CreateWidget` "/Game/SeddonsContent/UI/PickupUI/WBP_DS_Pickup_UI.WBP_DS_Pickup_UI_C"))
  (set `self.PickupUI` _returnvalue_2)
  ;[0.4072 0.04817 0.2542] Initialises Inventory UI
  (bind _returnvalue_3 (`|CreateWidget` "/Game/SeddonsContent/UI/InventoryUI/BPW_DS_Inventory_MenuUI.BPW_DS_Inventory_MenuUI_C"))
  (bind _output_get_2 (set `self.InventoryUI` _returnvalue_3))
  (`/Game/SeddonsContent/UI/InventoryUI/BPW_DS_Inventory_MenuUI.Initialise all Inventories` _output_get_2 (`/Game/SeddonsContent/Components/Items/Inventory.InventorySize` (`self.Inventory`))))

(event `EnhancedInput|/Game/SeddonsContent/Inputs/DefaultInputActions/IA_DS_OpenInventory`
  (params (ActionValue :type Boolean) (ElapsedSeconds :type "Float (double-precision)") (TriggeredSeconds :type "Float (double-precision)") (InputAction :type "InputAction Object Reference" :default "/Game/SeddonsContent/Inputs/DefaultInputActions/IA_DS_OpenInventory.IA_DS_OpenInventory"))
  (bind _returnvalue (`GameplayStatics.GetPlayerController` 0))
  (bind _inventoryui (`self.InventoryUI`))
  ;[0.4072 0.04817 0.2542] Open and closes the inventory UI
  (:`Started`
    (`/Engine/EditorBlueprintResources/StandardMacros.FlipFlop`
      (:`A`
        (`UserWidget.AddToViewport` _inventoryui 0)
        (set `PlayerController.bShowMouseCursor` true _returnvalue))
      (:`B`
        (`Widget.RemoveFromParent` _inventoryui)
        (set `PlayerController.bShowMouseCursor` false _returnvalue)))))

(event `EnhancedInput|/Game/SeddonsContent/Inputs/DefaultInputActions/IA_DS_Look`
  (params (ActionValue :type "Vector2D Structure") (ElapsedSeconds :type "Float (double-precision)") (TriggeredSeconds :type "Float (double-precision)") (InputAction :type "InputAction Object Reference" :default "/Game/SeddonsContent/Inputs/DefaultInputActions/IA_DS_Look.IA_DS_Look"))
  ;[0.4072 0.04817 0.2542] Allows for basic camera rotation
  (:`Triggered`
    (`self.AddControllerYawInput` ActionValue_X)
    (`self.AddControllerPitchInput` ActionValue_Y)))

(event `EnhancedInput|/Game/SeddonsContent/Inputs/DefaultInputActions/IA_DS_Move`
  (params (ActionValue :type "Vector2D Structure") (ElapsedSeconds :type "Float (double-precision)") (TriggeredSeconds :type "Float (double-precision)") (InputAction :type "InputAction Object Reference" :default "/Game/SeddonsContent/Inputs/DefaultInputActions/IA_DS_Move.IA_DS_Move"))
  ;[1 0.1159 0.6233] Allows for basic movement input
  (:`Triggered`
    (`self.AddMovementInput` (`self.GetActorRightVector`) ActionValue_X)
    (`self.AddMovementInput` (`self.GetActorForwardVector`) ActionValue_Y)))

(event `EnhancedInput|/Game/SeddonsContent/Inputs/DefaultInputActions/IA_DS_Sprint`
  (params (ActionValue :type Boolean) (ElapsedSeconds :type "Float (double-precision)") (TriggeredSeconds :type "Float (double-precision)") (InputAction :type "InputAction Object Reference" :default "/Game/SeddonsContent/Inputs/DefaultInputActions/IA_DS_Sprint.IA_DS_Sprint"))
  ;[0.4072 0.04817 0.2542] Allows the player to Sprint
  (:`Triggered`
    (if (and (`/Game/SeddonsContent/Components/Stats/Stamina.HasEnoughStamina` (`self.Stamina`) 1.0) (!= (`self.GetVelocity`) (0.0 0.0 0.0) :`ErrorTolerance` 0.01))
      (set `CharacterMovementComponent.MaxWalkSpeed` 600.0 (`self.CharacterMovement`))
      (`/Game/SeddonsContent/Components/Stats/Stamina.Start Stamina Drain` (`self.Stamina`))
      (else
        (`self.Stop Sprint`))))
  (:`Completed`
    (`self.Stop Sprint`)))

(event `EnhancedInput|/Game/SeddonsContent/Inputs/DefaultInputActions/IA_DS_Crouch`
  (params (ActionValue :type Boolean) (ElapsedSeconds :type "Float (double-precision)") (TriggeredSeconds :type "Float (double-precision)") (InputAction :type "InputAction Object Reference" :default "/Game/SeddonsContent/Inputs/DefaultInputActions/IA_DS_Crouch.IA_DS_Crouch"))
  ;[0.4072 0.04817 0.2542] Allows the player character to crouch
  (:`Triggered`
    (`self.Crouch`))
  (:`Completed`
    (`self.UnCrouch`)))

(event `Stop Sprint`
  ;[0.4072 0.04817 0.2542] Allows the player to Sprint
  (set `CharacterMovementComponent.MaxWalkSpeed` 400.0 (`self.CharacterMovement`))
  (`/Game/SeddonsContent/Components/Stats/Stamina.Cancel Stamina Drain` (`self.Stamina`)))

(event `self.Stamina.OnStaminaEmpty`
  ;[0.4072 0.04817 0.2542] Allows the player to Sprint
  (`self.Stop Sprint`))

(event `self.Stamina.OnStaminaChange`
  (params (`Current Stamina` :type "Float (double-precision)"))
  ;[0.4072 0.04817 0.2542] Allows the player to Sprint
  (`/Game/SeddonsContent/UI/GeneralUI/BPW_DS_StatBarUI.Update Stat Bar` (`/Game/SeddonsContent/UI/GeneralUI/BPW_DS_PlayerUI.StaminaBar` (`self.PlayerUI`)) `Current Stamina`))

(event `EnhancedInput|/Game/SeddonsContent/Inputs/DefaultInputActions/IA_DS_Dodge`
  (params (ActionValue :type Boolean) (ElapsedSeconds :type "Float (double-precision)") (TriggeredSeconds :type "Float (double-precision)") (InputAction :type "InputAction Object Reference" :default "/Game/SeddonsContent/Inputs/DefaultInputActions/IA_DS_Dodge.IA_DS_Dodge"))
  (bind (_returnvalue_x _returnvalue_y) (`KismetMathLibrary.BreakVector` (`self.GetVelocity`)))
  ;[0.4072 0.04817 0.2542] Allows the player to dash in the direction they're moving
  (:`Started`
    (if (and (`/Game/SeddonsContent/Components/Stats/Stamina.HasEnoughStamina` (`self.Stamina`) 20.0) (`NavMovementComponent.IsMovingOnGround` (`self.CharacterMovement`)))
      (if (!= (`self.GetVelocity`) (0.0 0.0 0.0))
        (`self.LaunchCharacter` (`KismetMathLibrary.MakeVector` (* _returnvalue_x 8.0) (* _returnvalue_y 8.0)) true true)
        (`/Game/SeddonsContent/Components/Stats/Stamina.Burst Stamina Loss` (`self.Stamina`) 20.0)))))

(event `Start Raycast`
  ;[0.4072 0.04817 0.2542] Cast a ray in the direction the player is looking to see if they are looking at something they can interact with
  (`KismetSystemLibrary.K2_SetTimerDelegate` (delegate `Cast a Ray`) 0.3 true))

(event `EnhancedInput|/Game/SeddonsContent/Inputs/DefaultInputActions/IA_DS_Interact`
  (params (ActionValue :type Boolean) (ElapsedSeconds :type "Float (double-precision)") (TriggeredSeconds :type "Float (double-precision)") (InputAction :type "InputAction Object Reference" :default "/Game/SeddonsContent/Inputs/DefaultInputActions/IA_DS_Interact.IA_DS_Interact"))
  (bind _lookatactor (`self.LookAtActor`))
  ;[0.402 0.04817 0.2542] Allows you to interact with and pick up objects
  (:`Started`
    (`/Engine/EditorBlueprintResources/StandardMacros.IsValid` _lookatactor
      (:`Is Valid`
        (if (`KismetSystemLibrary.DoesImplementInterface` _lookatactor "/Game/SeddonsContent/Items/BPI_DS_Item.BPI_DS_Item_C")
          (bind _pick_up (message `/Game/SeddonsContent/Items/BPI_DS_Item.Pickup` (`self.LookAtActor`)))
          (`/Game/SeddonsContent/Components/Items/Inventory.Add Item To Inventory` (`self.Inventory`) _pick_up 0 "NewEnumerator0")
          (message `/Game/SeddonsContent/Items/BPI_DS_Item.Picked Up` (`self.LookAtActor`))
          (set `self.LookAtActor` null))))))

(event `Cast a Ray`
  (bind _fp_cam (`self.FP_Cam`))
  (bind _returnvalue (`SceneComponent.K2_GetComponentLocation` _fp_cam))
  ;[0.4072 0.04817 0.2542] Cast a ray in the direction the player is looking to see if they are looking at something they can interact with
  (bind (_outhit _returnvalue_2) (`KismetSystemLibrary.SphereTraceSingleForObjects` _returnvalue (+ _returnvalue (* (`KismetMathLibrary.GetForwardVector` (`SceneComponent.K2_GetComponentRotation` _fp_cam)) 250.0)) 2.0 (`self.Object Types`)))
  (if _returnvalue_2
    (bind (_bblockinghit _binitialoverlap _time _distance _location _impactpoint _normal _impactnormal _physmat _hitactor) (`GameplayStatics.BreakHitResult` _outhit))
    (set `self.LookAtActor` _hitactor)
    (if (`KismetSystemLibrary.DoesImplementInterface` _hitactor "/Game/SeddonsContent/Items/BPI_DS_Item.BPI_DS_Item_C")
      (bind _pick_up (message `/Game/SeddonsContent/Items/BPI_DS_Item.Pickup` (`self.LookAtActor`)))
      (`/Game/SeddonsContent/UI/PickupUI/WBP_DS_PickupProfile.InitialiseProfile` (`/Game/SeddonsContent/UI/PickupUI/WBP_DS_Pickup_UI.PickUpItem` (`self.PickupUI`)) false (`.DataAsset_12_C9EFA92346799DB45436A88CC33AA459` (break `/Game/SeddonsContent/Items/DS_ItemStruct` _pick_up)))
      (`UserWidget.AddToViewport` (`self.PickupUI`) 0))
    (else
      (`Widget.RemoveFromParent` (`self.PickupUI`))
      (set `self.LookAtActor` null))))

(event `self.Inventory.OnEquippedItemChange`
  (params (`New Equipped Item` :type "/Game/SeddonsContent/Items/DS_ItemStruct Structure"))
  ;[0.4072 0.04817 0.2542] Spawns a new held item and attaches it to the player's hand
  (`/Engine/EditorBlueprintResources/StandardMacros.IsValid` (`self.HeldItem`)
    (:`Is Valid`
      (`self.K2_DestroyActor` (`self.HeldItem`)))
    (:`Is Not Valid`
      _))
  (bind (_helditem _success) (message `/Game/SeddonsContent/Items/BPI_DS_Item.HeldItem` (`.DataAsset_12_C9EFA92346799DB45436A88CC33AA459` (break `/Game/SeddonsContent/Items/DS_ItemStruct` `New Equipped Item`))))
  (if _success
    (bind _class (`|LoadAssetClass` _helditem)
      (:`Completed`
        (bind _asbp_ds_held_item_parent (castclass `/Game/SeddonsContent/Items/Blueprints/BP_DS_HeldItem_Parent` _class))
        (bind _returnvalue (`|SpawnActorFromClass` _asbp_ds_held_item_parent (`SceneComponent.K2_GetComponentToWorld` (`self.Test_Hand_Socket`)) "Undefined" "MultiplyWithRoot" null `New Equipped Item` null))
        (bind _output_get (set `self.HeldItem` _returnvalue))
        (`self.K2_AttachToComponent` _output_get (`self.Test_Hand_Socket`) "None" "SnapToTarget" "SnapToTarget" "KeepRelative" true)))))

(event `self.Inventory.OnPouchContentsChange`
  (params (Pouch :type "Map of Integer to /Game/SeddonsContent/Items/DS_ItemStruct Structure"))
  ;[0.4072 0.04817 0.2542] Spawns a new held item and attaches it to the player's hand
  (`/Game/SeddonsContent/UI/InventoryUI/BPW_DS_InventoryPanelUI.UpdateInventory` (`/Game/SeddonsContent/UI/GeneralUI/BPW_DS_PlayerUI.Pouch` (`self.PlayerUI`)) Pouch))

(event `self.Inventory.OnInventoryContentsChange`
  (params (Inventory :type "Map of Integer to /Game/SeddonsContent/Items/DS_ItemStruct Structure"))
  ;[0.4072 0.04817 0.2542] Spawns a new held item and attaches it to the player's hand
  (`/Game/SeddonsContent/UI/InventoryUI/BPW_DS_InventoryPanelUI.UpdateInventory` (`/Game/SeddonsContent/UI/InventoryUI/BPW_DS_Inventory_MenuUI.MainInventory` (`self.InventoryUI`)) Inventory))

(event `self.Health.OnDamageTaken`
  (params (`Current Health` :type "Float (double-precision)"))
  (`/Game/SeddonsContent/UI/GeneralUI/BPW_DS_StatBarUI.Update Stat Bar` (`/Game/SeddonsContent/UI/GeneralUI/BPW_DS_PlayerUI.HealthBar` (`self.PlayerUI`)) `Current Health`))

(event `self.Mana.OnManaChange`
  (params (`Current Mana` :type "Float (double-precision)"))
  (`/Game/SeddonsContent/UI/GeneralUI/BPW_DS_StatBarUI.Update Stat Bar` (`/Game/SeddonsContent/UI/GeneralUI/BPW_DS_PlayerUI.ManaBar` (`self.PlayerUI`)) `Current Mana`))

(fn `UserConstructionScript`)