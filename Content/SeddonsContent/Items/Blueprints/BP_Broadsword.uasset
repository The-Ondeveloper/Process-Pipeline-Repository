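; BP_Broadsword is a held melee weapon that damages what it hits on primary input.
; When triggered off cooldown, it runs a zero-length sphere trace at AttackArrow, with debug drawing, and applies damage to the hit actor.
; Radius, damage and timer delay come from the item's data asset stats, scaled by per-item modifiers.
; Each swing, hit or miss, sets Cooldown and starts the speed-based timer.
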(event `/Game/SeddonsContent/Inputs/BPI_DS_Inputs.HeldItemPrimaryInput`
  (params (ActionType :type "/Game/SeddonsContent/Inputs/EInputTriggerState Enum" :default "NewEnumerator0"))
  (bind ((`DataAsset_12_C9EFA92346799DB45436A88CC33AA459` _dataasset) (`SpeedModifier_7_9FE375434C9770295BBA6C9523DDEE1C` _speedmodifier)) (break `/Game/SeddonsContent/Items/DS_ItemStruct` (`self.Item Data`)))
  (bind ((`DataAsset_12_C9EFA92346799DB45436A88CC33AA459` _dataasset_2) (`SizeModifier_9_CED41F0F43F0F5D8DD3F0283323EF8B1` _sizemodifier)) (break `/Game/SeddonsContent/Items/DS_ItemStruct` (`self.Item Data`)))
  (bind ((`DataAsset_12_C9EFA92346799DB45436A88CC33AA459` _dataasset_3) (`DamageModifier_3_A76E35094C802706CE3C6A8FAFC26272` _damagemodifier)) (break `/Game/SeddonsContent/Items/DS_ItemStruct` (`self.Item Data`)))
  (bind _returnvalue (`SceneComponent.K2_GetComponentLocation` (`self.AttackArrow`)))
  (switch `/Game/SeddonsContent/Inputs/EInputTriggerState` ActionType
    (:`NewEnumerator0`
      (if (not (`self.Cooldown`))
        (bind (_damage _staminacost _speed _collisionsize) (message `/Game/SeddonsContent/Items/BPI_DS_Item.Get Stats` _dataasset_2))
        (bind (_outhit _returnvalue_2) (`KismetSystemLibrary.SphereTraceSingleForObjects` :`Start` _returnvalue :`End` _returnvalue :`Radius` (* _collisionsize _sizemodifier) :`ObjectTypes` (`self.Object Types`) :`DrawDebugType` "ForDuration"))
        (`|ExecutionSequence`
          (:`then_0`
            (if _returnvalue_2
              (bind _damage_2 (message `/Game/SeddonsContent/Items/BPI_DS_Item.Get Stats` _dataasset_3))
              (`GameplayStatics.ApplyDamage` (`.HitActor` (`GameplayStatics.BreakHitResult` _outhit)) (* _damage_2 _damagemodifier))))
          (:`then_1`
            (set `self.Cooldown` true)
            (bind (_damage_3 _staminacost_2 _speed_2) (message `/Game/SeddonsContent/Items/BPI_DS_Item.Get Stats` _dataasset))
            (`KismetSystemLibrary.K2_SetTimerDelegate` (`|CreateDelegate` :!event `Reset cooldown`) (* _speed_2 _speedmodifier))))))))

(fn `UserConstructionScript`
  (`parent.UserConstructionScript`))