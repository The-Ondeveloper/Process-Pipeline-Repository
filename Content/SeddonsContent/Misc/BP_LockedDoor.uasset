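; BP_LockedDoor is an interactable double door that stays shut until the interacting actor's inventory holds the required key.
; Interact sets each door's unlock flag by inventory lookup, though both sides search for "Key [L]", and prints a warning on failure.
; A success fires OnUnlocked; once both flags are set, its handler disables box collision and a timeline rotates both doors open.
; Other item functions are stubs, except the "Locked Doors" label.
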(event `self.ReceiveBeginPlay`
  (add `self.OnUnlocked` (delegate `UnlockDoors`)))

(event `UnlockDoors`
  (if (and (`self.LeftDoorOpen`) (`self.RightDoorOpen`))
    (`PrimitiveComponent.SetCollisionEnabled` (`self.Box Collision`) "NoCollision")
    (bind (_direction _time) (`Timeline|OpenSesame`)
      (:`Update`
        (`SceneComponent.K2_SetRelativeRotation` (`self.DoorR`) (`KismetMathLibrary.RLerp` (`SceneComponent.RelativeRotation` (`self.DoorR`)) (struct :`Yaw` -85.0) _time true) false false)
        (`SceneComponent.K2_SetRelativeRotation` (`self.DoorL`) (`KismetMathLibrary.RLerp` (`SceneComponent.RelativeRotation` (`self.DoorL`)) (struct :`Yaw` -85.0) _time true) false false))
      (:`Finished`
        (set `self.DoorOpen` true)))))

(event `/Game/SeddonsContent/Misc/BPI_Interact.Interact`
  (params (Sender :type "/Game/SeddonsContent/PlayerCharacter/BP_DS_Playercharacter Object Reference"))
  (`|ExecutionSequence`
    (:`then_0`
      (if (not (`self.LeftDoorOpen`))
        (bind _return_value (`/Game/SeddonsContent/Components/Items/Inventory.Find First Instance of Item by Name ` (`/Game/SeddonsContent/PlayerCharacter/BP_DS_Playercharacter.Inventory` Sender) "Key [L]"))
        (bind _output_get (set `self.LeftDoorOpen` _return_value))
        (if _output_get
          (`self.OnUnlocked`)
          (else
            (`KismetSystemLibrary.PrintString` "Key(s) Missing!" :!label _label)))))
    (:`then_1`
      (if (not (`self.RightDoorOpen`))
        (bind _return_value_2 (`/Game/SeddonsContent/Components/Items/Inventory.Find First Instance of Item by Name ` (`/Game/SeddonsContent/PlayerCharacter/BP_DS_Playercharacter.Inventory` Sender) "Key [L]"))
        (bind _output_get_2 (set `self.RightDoorOpen` _return_value_2))
        (if _output_get_2
          (`self.OnUnlocked`)
          (else
            (goto _label)))))))

(fn `Get Object Details`
  (returns (`Object Name` :type Text))
  (return "Locked Doors"))

(fn `Get Stats`
  (returns (Damage :type "Float (double-precision)") (StaminaCost :type "Float (double-precision)") (Speed :type "Float (double-precision)") (CollisionSize :type "Float (double-precision)"))
  (return 0.0 0.0 0.0 0.0))

(fn `HeldItem`
  (returns (HeldItem :type "/Game/SeddonsContent/Items/Blueprints/BP_DS_HeldItem_Parent Soft Class Reference") (Success :type Boolean))
  (return null false))

(fn `Pickup`
  (returns (`Pick Up` :type "/Game/SeddonsContent/Items/DS_ItemStruct Structure"))
  (return))

(fn `UserConstructionScript`)