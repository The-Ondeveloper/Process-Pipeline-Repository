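; Parent component for held items that provides the shared primary-action input handling.
; On BeginPlay it adds the held-item Enhanced Input mapping context to player 0's subsystem at priority 1, if not already present.
; Each trigger phase of the primary item action is forwarded through HeldItemPrimaryInputMessage as a distinct enum value.
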(event `self.ReceiveBeginPlay`
  (bind _returnvalue (pcsubsystem `EnhancedInputLocalPlayerSubsystem` (`GameplayStatics.GetPlayerController` 0)))
  (`/Engine/EditorBlueprintResources/StandardMacros.IsValid` _returnvalue
    (:`Is Valid`
      (if (not (`.ReturnValue` (`EnhancedInputSubsystemInterface.HasMappingContext` _returnvalue "/Game/SeddonsContent/Inputs/IMC_DS_HeldItems.IMC_DS_HeldItems")))
        (`EnhancedInputSubsystemInterface.AddMappingContext` _returnvalue "/Game/SeddonsContent/Inputs/IMC_DS_HeldItems.IMC_DS_HeldItems" 1 (struct))))))

(event `EnhancedInput|/Game/SeddonsContent/Inputs/DefaultInputActions/IA_DS_Item_Primary`
  (params (ActionValue :type Boolean) (ElapsedSeconds :type "Float (double-precision)") (TriggeredSeconds :type "Float (double-precision)") (InputAction :type "InputAction Object Reference" :default "/Game/SeddonsContent/Inputs/DefaultInputActions/IA_DS_Item_Primary.IA_DS_Item_Primary"))
  (:`Triggered`
    (message `/Game/SeddonsContent/Inputs/BPI_DS_Inputs.HeldItemPrimaryInput` self "NewEnumerator0"))
  (:`Started`
    (message `/Game/SeddonsContent/Inputs/BPI_DS_Inputs.HeldItemPrimaryInput` self "NewEnumerator1"))
  (:`Ongoing`
    (message `/Game/SeddonsContent/Inputs/BPI_DS_Inputs.HeldItemPrimaryInput` self "NewEnumerator2"))
  (:`Canceled`
    (message `/Game/SeddonsContent/Inputs/BPI_DS_Inputs.HeldItemPrimaryInput` self "NewEnumerator3"))
  (:`Completed`
    (message `/Game/SeddonsContent/Inputs/BPI_DS_Inputs.HeldItemPrimaryInput` self "NewEnumerator4")))