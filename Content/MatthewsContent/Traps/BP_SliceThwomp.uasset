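; BP_SliceThwomp is a trap that bobs up and down and damages actors that touch it.
; BeginPlay caches the mesh's relative Z, and Tick offsets it with a sine of game time scaled by speed and distance variables.
; Overlapping the collision component applies fixed damage to the other actor and prints a debug message.
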(event `self.ReceiveBeginPlay`
  (set `self.RelativeStartingLocationZ` (.z (.location (`SceneComponent.GetRelativeTransform` (`self.StaticMesh`))))))

(event `self.ReceiveTick`
  (params (DeltaSeconds :type "Float (single-precision)"))
  (`SceneComponent.K2_SetRelativeLocation` (`self.StaticMesh`) (`KismetMathLibrary.MakeVector` 0.0 0.0 (+ (`self.RelativeStartingLocationZ`) (* (`KismetMathLibrary.DegSin` (* (`self.GetGameTimeSinceCreation`) (`self.BobbingSpeed`))) (`self.BobbingDistance`)))) false false))

(event `self.Collision.OnComponentBeginOverlap`
  (params (OverlappedComponent :type "PrimitiveComponent Object Reference") (OtherActor :type "Actor Object Reference") (OtherComp :type "PrimitiveComponent Object Reference") (OtherBodyIndex :type Integer) (bFromSweep :type Boolean) (SweepResult :type "HitResult Structure (by ref)"))
  (`GameplayStatics.ApplyDamage` OtherActor 20.0)
  (`KismetSystemLibrary.PrintText` "Sliced"))

(fn `UserConstructionScript`)