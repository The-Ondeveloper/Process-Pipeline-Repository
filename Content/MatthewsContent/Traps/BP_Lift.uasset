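; BP_Lift is a trap-folder actor whose static mesh continuously bobs up and down along its local Z axis.
; BeginPlay caches the mesh's starting relative Z.
; Each Tick offsets that Z by a degree-based sine of game time since creation, scaled by BobbingSpeed and BobbingDistance.
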(event `self.ReceiveBeginPlay`
  (set `self.RelativeStartingLocationZ` (.z (.location (`SceneComponent.GetRelativeTransform` (`self.StaticMesh`))))))

(event `self.ReceiveTick`
  (params (DeltaSeconds :type "Float (single-precision)"))
  (`SceneComponent.K2_SetRelativeLocation` (`self.StaticMesh`) (`KismetMathLibrary.MakeVector` 0.0 0.0 (+ (`self.RelativeStartingLocationZ`) (* (`KismetMathLibrary.DegSin` (* (`self.GetGameTimeSinceCreation`) (`self.BobbingSpeed`))) (`self.BobbingDistance`)))) false false))

(fn `UserConstructionScript`)